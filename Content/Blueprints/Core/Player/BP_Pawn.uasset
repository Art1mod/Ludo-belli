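; BP_Pawn is a player-controlled camera pawn with zoom, planar movement and yaw rotation through Enhanced Input.
; BeginPlay adds the base mapping context, and input events update desired zoom, location and rotation, with zoom clamped and movement relative to the actor's forward and right vectors.
; Tick smoothly interpolates spring arm length and actor transform toward those targets, which the construction script seeds from initial values.
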(event `self.ReceiveTick`
  (params (DeltaSeconds :type "Float (single-precision)"))
  ;[0.02187 0.02187 0.02187] Camera update
  (set `SpringArmComponent.TargetArmLength` (`KismetMathLibrary.FInterpTo` (`SpringArmComponent.TargetArmLength` (`self.SpringArm`)) (`self.DesiredZoom`) DeltaSeconds 2.0) (`self.SpringArm`))
  (`self.K2_SetActorLocation` (`KismetMathLibrary.VInterpTo` (`self.K2_GetActorLocation`) (`self.DesiredLocation`) DeltaSeconds 5.0))
  (`self.K2_SetActorRotation` (`KismetMathLibrary.RInterpTo` (`self.K2_GetActorRotation`) (`self.DesiredRotator`) DeltaSeconds 2.5)))

(event `self.ReceiveBeginPlay`
  ;[0.01444 0.01444 0.01444] Setting Input Mapping Context
  (bind _asplayer_controller (cast `PlayerController` (`self.GetController`)))
  (`EnhancedInputSubsystemInterface.AddMappingContext` (pcsubsystem `EnhancedInputLocalPlayerSubsystem` _asplayer_controller) "/Game/Blueprints/Core/Input/IMC_Base.IMC_Base" 0 (struct)))

(event `EnhancedInput|/Game/Blueprints/Core/Input/IA_Zoom`
  (params (ActionValue :type "Float (double-precision)") (ElapsedSeconds :type "Float (double-precision)") (TriggeredSeconds :type "Float (double-precision)") (InputAction :type "InputAction Object Reference" :default "/Game/Blueprints/Core/Input/IA_Zoom.IA_Zoom"))
  ;[0.009721 0.009721 0.009721] Inputs
  (:`Triggered`
    (set `self.DesiredZoom` (`KismetMathLibrary.FClamp` (+ (* (* ActionValue -1.0) 80.0) (`self.DesiredZoom`)) 500.0 2000.0))))

(event `EnhancedInput|/Game/Blueprints/Core/Input/IA_Move`
  (params (ActionValue :type "Vector2D Structure") (ElapsedSeconds :type "Float (double-precision)") (TriggeredSeconds :type "Float (double-precision)") (InputAction :type "InputAction Object Reference" :default "/Game/Blueprints/Core/Input/IA_Move.IA_Move"))
  ;[0.009721 0.009721 0.009721] Inputs
  (:`Triggered`
    (set `self.DesiredLocation` (+ (* (* ActionValue_X 20.0) (`self.GetActorRightVector`)) (`self.DesiredLocation`)))
    (set `self.DesiredLocation` (+ (* (* ActionValue_Y 30.0) (`self.GetActorForwardVector`)) (`self.DesiredLocation`)))))

(event `EnhancedInput|/Game/Blueprints/Core/Input/IA_Rotate`
  (params (ActionValue :type "Float (double-precision)") (ElapsedSeconds :type "Float (double-precision)") (TriggeredSeconds :type "Float (double-precision)") (InputAction :type "InputAction Object Reference" :default "/Game/Blueprints/Core/Input/IA_Rotate.IA_Rotate"))
  ;[0.009721 0.009721 0.009721] Inputs
  (:`Triggered`
    (set `self.DesiredRotator` (`KismetMathLibrary.ComposeRotators` (`self.DesiredRotator`) (`KismetMathLibrary.MakeRotator` 0.0 0.0 (* ActionValue 45.0))))))

(fn `UserConstructionScript`
  (set `self.DesiredZoom` (`SpringArmComponent.TargetArmLength` (`self.SpringArm`)))
  (set `self.DesiredLocation` (`self.K2_GetActorLocation`))
  (set `self.DesiredRotator` (`self.K2_GetActorRotation`)))